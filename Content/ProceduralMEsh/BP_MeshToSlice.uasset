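; BP_MeshToSlice is an actor whose mesh is cut by whatever component overlaps it.
; The construction script and BeginPlay both copy the static mesh into a procedural mesh with collision.
; On overlap, it slices along the other component's location and up vector, capping the cut with a new section.
; The resulting half is sliced again on the same plane, and that output gets physics simulation.
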(event OnComponentBeginOverlap(ProceduralMesh)
  (params (OverlappedComponent :type Primitive%20Component%20Object%20Reference) (OtherActor :type Actor%20Object%20Reference) (OtherComp :type Primitive%20Component%20Object%20Reference) (OtherBodyIndex :type Integer) (bFromSweep :type Boolean) (SweepResult :type Hit%20Result%20Structure%20%28by%20ref%29))
  (bind _returnvalue (Transformation|GetWorldLocation OtherComp))
  (bind _returnvalue_2 (Math|Vector|GetUpVector OtherComp))
  (bind _outotherhalfprocmesh (Class|KismetProceduralMeshLibrary|SliceProceduralMesh (Variables|Default|GetProceduralMesh) _returnvalue _returnvalue_2 true "CreateNewSectionForCap" "/Engine/MapTemplates/Materials/BasicAsset01.BasicAsset01"))
  (bind _outotherhalfprocmesh_2 (Class|KismetProceduralMeshLibrary|SliceProceduralMesh _outotherhalfprocmesh _returnvalue _returnvalue_2 true "CreateNewSectionForCap"))
  (Physics|SetSimulatePhysics _outotherhalfprocmesh_2 true))

(event Collision|EventActorBeginOverlap
  (params (OtherActor :type Actor%20Object%20Reference)))

(event EventTick
  (params (DeltaSeconds :type Float%20%28single-precision%29)))

(event EventBeginPlay
  (Class|KismetProceduralMeshLibrary|CopyProceduralMeshfromStaticMeshComponent (Variables|Default|GetStaticMesh) 0 (Variables|Default|GetProceduralMesh) true))

(fn ConstructionScript
  (Class|KismetProceduralMeshLibrary|CopyProceduralMeshfromStaticMeshComponent (Variables|Default|GetStaticMesh) 0 (Variables|Default|GetProceduralMesh) true))